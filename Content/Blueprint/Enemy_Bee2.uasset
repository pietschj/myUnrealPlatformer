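; Bee enemy that moves its body vertically on a timeline, shoots the player on sight and dies when its health runs out.
; PawnSensing makes it face the player and start a looping fire timer, both cancelled by a retriggerable delay once sightings stop.
; Each shot is a debug-drawn forward line trace with random upward offset for misses, applying damage and briefly swapping gun particle systems.
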(event OnSeePawn(PawnSensing)
  (params (Pawn :type Pawn%20Object%20Reference))
  ;[1 1 1] PawnSensing set shouldRotate boolean
  (Variables|Default|SetshouldRotate true)
  (CallFunction|ShootPlayer)
  (Utilities|FlowControl|RetriggerableDelay 4.0)
  (Variables|Default|SetshouldRotate false)
  ;[1 1 1] reset ShootEvent
  (Utilities|Time|ClearandInvalidateTimerbyHandle (Variables|Default|GetshootEvent))
  (CallFunction|ResetDoOnce))

(event Custom|ShootPlayer
  ;[1 1 1] shootPlayer custom Funciton
  (Utilities|FlowControl|DoOnce false
    (:Completed
      (bind _returnvalue (Utilities|Time|SetTimerbyEvent (delegate Custom|shoot) (Variables|Default|GetFirerate) true))
      (Variables|Default|SetshootEvent _returnvalue))))

(event Custom|shoot
  (bind _returnvalue (Transformation|GetActorLocation))
  ;[1 1 1] shootPlayer custom Funciton
  (Audio|PlaySoundatLocation "/Game/imported/Kenny/sounds/enemy_attack.enemy_attack" (Transformation|GetActorLocation) "0, 0, 0" 1.0 1.0 0.0 0 0 0 0)
  ;[1 1 1] LineTrace EnemyForward
  (bind _outhit (Collision|LineTraceByChannel _returnvalue (+ (+ _returnvalue (* (Math|Vector|GetForwardVector (Transformation|GetActorRotation)) (Variables|Default|GetfireDistance))) (Math|Vector|MakeVector 0.0 0.0 (Math|Random|RandomFloatinRange 0.0 5e+02))) "TraceTypeQuery1" false 0 "ForDuration"))
  (Game|Damage|ApplyDamage (.HitActor (Collision|BreakHitResult _outhit)) 1.0 0 0)
  ;[1 1 1] apply particles to enemy guns
  (Class|NiagaraComponent|SetAsset (Variables|Default|Getparticles) "/Game/Particles/Enemy1_system.Enemy1_system" true)
  (Utilities|FlowControl|Delay 0.2)
  (Class|NiagaraComponent|SetAsset (Variables|Default|Getparticles) "/Game/Particles/Enemy2_System.Enemy2_System" true))

(event Custom|reset%20doOnce
  ;[1 1 1] shootPlayer custom Funciton
  (Utilities|FlowControl|DoOnce false) ; enters at Reset
)

(event EventBeginPlay
  (bind _enemybody (Variables|Default|GetenemyBody))
  (bind _relativelocation (Variables|/Script/Engine.SceneComponent|GetRelativeLocation _enemybody))
  ;[1 1 1] EnemyAnimation
  (bind _enemymovement (Timeline|Timeline Play)
    (:Update
      (Transformation|SetRelativeLocation _enemybody (Math|Vector|MakeVector (.x _relativelocation) (.y _relativelocation) (Math|Float|Lerp 0.0 (Variables|Default|GetenemyMovementDistance) _enemymovement)) false false))))

(event Collision|EventActorBeginOverlap
  (params (OtherActor :type Actor%20Object%20Reference)))

(event EventTick
  (params (DeltaSeconds :type Float%20%28single-precision%29))
  ;[1 1 1] EnemyRotates if PawnSensing detects Player
  (if (Variables|Default|GetshouldRotate)
    (Transformation|SetActorRotation (Math|Rotator|FindLookatRotation (Transformation|GetActorLocation) (Transformation|GetActorLocation (Game|GetPlayerCharacter 0))))))

(event Game|Damage|EventAnyDamage
  (params (Damage :type Float%20%28single-precision%29) (DamageType :type Damage%20Type%20Object%20Reference) (InstigatedBy :type Controller%20Object%20Reference) (DamageCauser :type Actor%20Object%20Reference))
  ;[1 1 1] Enemy Damage System
  (bind _output_get (Variables|Default|SetHealth (- (Variables|Default|GetHealth) Damage)))
  (if (<= _output_get 0.0)
    (Audio|PlaySoundatLocation "/Game/imported/Kenny/sounds/enemy_destroy.enemy_destroy" (Transformation|GetActorLocation) "0, 0, 0" 1.0 1.0 0.0 0 0 0 0)
    (Actor|DestroyActor)
    (else
      (Audio|PlaySoundatLocation "/Game/imported/Kenny/sounds/enemy_hurt.enemy_hurt" (Transformation|GetActorLocation) "0, 0, 0" 1.0 1.0 0.0 0 0 0 0))))

(fn ConstructionScript)